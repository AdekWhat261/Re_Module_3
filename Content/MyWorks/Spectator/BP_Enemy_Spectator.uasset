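; BP_Enemy_Spectator is an enemy that watches the player, tracking an Alert value based on line of sight.
; Each tick it traces on Visibility to the player character, treating a hit as hidden and no hit as seen.
; Alert drains, clamped, while hidden and rises while seen, with debug prints.
; Every seen tick calls Open Level for SecondMap; the Alert threshold only feeds its Absolute flag, without gating the call.
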(event EventTick
  (params (DeltaSeconds :type Float%20%28single-precision%29))
  (bind _returnvalue (Collision|LineTraceByChannel (Transformation|GetActorLocation) (Transformation|GetActorLocation (Game|GetPlayerCharacter 0)) "TraceTypeQuery1" false 0 "ForDuration" true "(R=0.000000,G=1.000000,B=0.179629,A=1.000000)" "(R=1.000000,G=0.018841,B=0.078564,A=1.000000)"))
  (if _returnvalue
    (Development|PrintString "Hidden" true true "(R=1.000000,G=0.000000,B=0.078579,A=1.000000)" 0.0)
    (bind _output_get (Variables|Default|SetAlert (Math|Float|Clamp(Float) (- (Variables|Default|GetAlert) DeltaSeconds) 0.0 5.0)))
    (Development|PrintString (Utilities|String|ToString(Float) _output_get) true true "(R=1.000000,G=0.038562,B=0.000000,A=1.000000)" 0.0)
    (else
      (Development|PrintString "Seen" true true "(R=0.000000,G=1.000000,B=0.066792,A=1.000000)" 0.0)
      (bind _output_get_2 (Variables|Default|SetAlert (+ (Variables|Default|GetAlert) DeltaSeconds)))
      (Development|PrintString (Utilities|String|ToString(Float) _output_get_2) true true "(R=0.000000,G=1.000000,B=0.128237,A=1.000000)" 0.0)
      (Game|OpenLevel(byObjectReference) "/Game/FirstPerson/Maps/SecondMap.SecondMap" (>= _output_get_2 5.0)))))

(fn ConstructionScript)