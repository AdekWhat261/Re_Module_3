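; Shotgun weapon Blueprint that fires a spread of hitscan pellets when ready.
; Shoot line-traces each pellet from the muzzle toward a camera-forward point randomly offset per axis, with debug drawing.
; Hit actors take damage, and BP_ParentEnemy targets also receive a hit event.
; A separate Reloading event blocks firing for the pump delay; projectile-spawn logic is left unconnected.
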(event Custom|Shoot
  (bind _returnvalue (Game|GetPlayerCameraManager 0))
  (bind _scatter__antiaccuracy_ (Variables|Default|GetScatter%20%28antiAccuracy%29))
  (bind _returnvalue_2 (* _scatter__antiaccuracy_ -1))
  ;[0.2622 0.2622 0.2622] Не находится ли дробовик в перезарядке
  (if (Variables|Default|GetIsReadyToShoot)
    (for _index (range 0 (Variables|Default|GetNum%20of%20Pellets)) ; Кол-во дробинок (выпускаемые лайнтрейсы)
      (bind _outhit (Collision|LineTraceByChannel (Transformation|GetSocketLocation (Variables|ObjectReferences|GetSK_FPGun) "Muzzle") (+ (+ (Camera|GetCameraLocation _returnvalue) (* (Transformation|GetActorForwardVector _returnvalue) (Variables|Default|GetDistance))) (Math|Vector|MakeVector (Math|Random|RandomFloatinRange _returnvalue_2 _scatter__antiaccuracy_) (Math|Random|RandomFloatinRange _returnvalue_2 _scatter__antiaccuracy_) (Math|Random|RandomFloatinRange _returnvalue_2 _scatter__antiaccuracy_))) "TraceTypeQuery3" false 0 "ForDuration" true "(R=0.327155,G=1.000000,B=0.160002,A=1.000000)" "(R=1.000000,G=0.058617,B=0.085147,A=1.000000)" 0.5))
      (Game|Damage|ApplyDamage (.HitActor (Collision|BreakHitResult _outhit)) 5e+01 0 0)
      (bind _asbp_parent_enemy (Utilities|Casting|CastToBP_ParentEnemy (.HitActor (Collision|BreakHitResult _outhit))))
      (Default|CustomEventHit _asbp_parent_enemy))))

(event Custom|Reloading
  ;[0.02951 0.02951 0.02951] Перезарядка (после каждого выстрела)
  (Variables|Default|SetIsReadyToShoot false)
  (Utilities|FlowControl|Delay (Variables|Default|GetDelay,%20pump%20reload))
  (Variables|Default|SetIsReadyToShoot true))

(fn ConstructionScript)